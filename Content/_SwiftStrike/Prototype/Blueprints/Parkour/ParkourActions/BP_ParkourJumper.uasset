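; BP_ParkourJumper is a prototype parkour action, named for jumping, that currently adds no jump logic of its own.
; PerformSkill calls its parent and then GetParkourCharacter without using the result.
; SetParkourManager and both getters simply forward to the parent class.
; An unconnected debug chain would print the character's mid-air time through BPI_ParkourCharacter, but it never runs.
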(event EventPerformSkill
  (|CallParentFunction)
  (CallFunction|GetParkourCharacter))

(event EventSetParkourManager
  (params (ParkourManager :type BP%20SS%20Parkour%20Manager%20Component%20Object%20Reference))
  (|CallParentFunction ParkourManager))

(fn ConstructionScript)

(fn GetParkourManager
  (bind _parkourmanager (|CallParentFunction))
  (return _parkourmanager))

(fn GetParkourCharacter
  (bind _parkourcharacter (|CallParentFunction))
  (return _parkourcharacter))