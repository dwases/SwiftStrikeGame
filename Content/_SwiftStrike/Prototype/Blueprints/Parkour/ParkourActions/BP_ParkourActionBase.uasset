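; Base Blueprint for parkour actions, with an empty PerformSkill event.
; It stores a ParkourManager reference passed in through SetParkourManager and exposes it through a getter.
; GetParkourCharacter casts that manager's owner to BPI_ParkourCharacter, printing and logging an error if the owner does not implement the interface.
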(event EventPerformSkill)

(event EventSetParkourManager
  (params (ParkourManager :type BP%20SS%20Parkour%20Manager%20Component%20Object%20Reference))
  (Variables|Default|SetParkourManager ParkourManager))

(fn ConstructionScript)

(fn GetParkourCharacter
  (bind _returnvalue (Utilities|String|MakeLiteralString "ParkourManager's owner needs to implement BPI_ParkourCharacter"))
  (bind _parkourmanager (CallFunction|GetParkourManager))
  (bind _asbpi_parkour_character (Utilities|Casting|CastToBPI_ParkourCharacter (Components|GetOwner _parkourmanager))
    (:then
      (return _asbpi_parkour_character))
    (:CastFailed
      (Development|PrintString _returnvalue)
      (Utilities|String|LogString _returnvalue))))

(fn GetParkourManager
  (return (Variables|Default|GetParkourManager)))